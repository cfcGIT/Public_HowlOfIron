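; Rain effect actor that builds a tiled grid of Niagara rain emitters and plays 2D rain and alarm sounds.
; InitPlay spawns and centers the grid on construction and BeginPlay, applying RainType presets or custom values as Niagara parameters.
; Every 0.2 seconds, Tick traces upward from the werewolf and drops the following component's Z offset under cover, restoring it in open sky.
; Events adjust rain volume for normal play and cutscenes.
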(event `self.ReceiveBeginPlay`
  (`self.InitPlay`)
  (`self.BeginRain`)
  (`self.SetActorTickEnabled` true))

(event `self.ReceiveTick`
  (params (DeltaSeconds :type "Float (single-precision)"))
  (bind _hifollowing (`self.HIFollowing`))
  (bind _hifollowing_2 (`self.HIFollowing`))
  (bind (_offset_x _offset_y) (`KismetMathLibrary.BreakVector` (`HIFollowingComponent.offset` _hifollowing)))
  (bind (_offset_x_2 _offset_y_2) (`KismetMathLibrary.BreakVector` (`HIFollowingComponent.offset` _hifollowing_2)))
  (bind _output_get (set `self.timerDePablo` (+ DeltaSeconds (`self.timerDePablo`))))
  (if (> _output_get 0.2)
    (set `self.timerDePablo` 0.0)
    (bind _returnvalue (`HIGameData.HIGetWerewolfLocation`))
    (bind (_outhit _returnvalue_2) (`KismetSystemLibrary.LineTraceSingle` (`KismetMathLibrary.MakeVector` (.x _returnvalue) (.y _returnvalue) (+ (.z _returnvalue) 200.0)) (`KismetMathLibrary.MakeVector` (.x _returnvalue) (.y _returnvalue) (+ (.z _returnvalue) 4000.0)) "TraceTypeQuery1"))
    (if _returnvalue_2
      (for _array_element (`self.Niagara`)
        (`/Engine/EditorBlueprintResources/StandardMacros.IsValid` _array_element
          (:`Is Valid`
            (set `HIFollowingComponent.offset` (`KismetMathLibrary.MakeVector` _offset_x_2 _offset_y_2 (+ 0.0 -3000.0)) _hifollowing_2))))
      (else
        (for _array_element_2 (`self.Niagara`)
          (`/Engine/EditorBlueprintResources/StandardMacros.IsValid` _array_element_2
            (:`Is Valid`
              (set `HIFollowingComponent.offset` (`KismetMathLibrary.MakeVector` _offset_x _offset_y) _hifollowing))))))))

(event `BeginRain`
  (bind _returnvalue (`GameplayStatics.SpawnSound2D` "/Game/Game_Files/SFX/SoundsFinal/Ambient/Rain/SC_Rain_Light_1_Cue.SC_Rain_Light_1_Cue" 1.0 1.0 0.0 null))
  (set `self.RainSound` _returnvalue))

(event `NormalRain`
  (`AudioComponent.SetVolumeMultiplier` (`self.RainSound`) 1.0))

(event `CutsceneRain`
  (`/Engine/EditorBlueprintResources/StandardMacros.IsValid` (`self.RainSound`)
    (:`Is Valid`
      _)
    (:`Is Not Valid`
      (bind _returnvalue (`GameplayStatics.SpawnSound2D` "/Game/Game_Files/SFX/SoundsFinal/Ambient/Rain/SC_Rain_Light_1_Cue.SC_Rain_Light_1_Cue" 1.0 1.0 0.0 null))
      (set `self.RainSound` _returnvalue)))
  (`AudioComponent.SetVolumeMultiplier` (`self.RainSound`) 0.5))

(event `BeginAlarm`
  (bind _returnvalue (`GameplayStatics.SpawnSound2D` "/Game/Game_Files/SFX/SoundsFinal/Ambient/FactoryAlarms/SFX_Alarm_Cue.SFX_Alarm_Cue" 1.0 1.0 0.0 null))
  (set `self.AlarmSound` _returnvalue))

(fn `InitPlay`
  (bind _rain (`self.rain`))
  (bind _velocity (`self.velocity`))
  (bind _rain_type (`self.Rain_Type`))
  (bind _rain_2 (`self.rain`))
  (bind _rain_3 (`self.rain`))
  (bind _rain_4 (`self.rain`))
  (bind _rain_5 (`self.rain`))
  (bind _rain_6 (`self.rain`))
  (bind _area (`self.Area`))
  (bind (_r _g _b) (break `LinearColor` (`self.Color`)))
  (bind (_x _y) (`KismetMathLibrary.BreakVector2D` (`self.Tile`)))
  (bind (_x_2 _y_2) (`KismetMathLibrary.BreakVector2D` (`self.Tile`)))
  (`KismetArrayLibrary.Array_Clear` (`self.Niagara`))
  (for _index (range 1 (+ (`KismetMathLibrary.FTrunc` (* (`KismetMathLibrary.Abs` _x) (`KismetMathLibrary.Abs` _y))) 1))
    (bind _returnvalue (`AddComponent|NODE_AddNiagaraComponent-0` :`RelativeTransform` (`KismetMathLibrary.MakeTransform` (0.0 0.0 0.0))))
    (`KismetArrayLibrary.Array_Set` (`self.Niagara`) _index _returnvalue true))
  (for (_array_element _array_index) (`self.Niagara`)
    (if (`KismetSystemLibrary.IsValid` _array_element)
      (bind _returnvalue_2 (mod _array_index (`KismetMathLibrary.FTrunc` (`KismetMathLibrary.Abs` (`KismetMathLibrary.BreakVector2D` (`self.Tile`))))))
      (`SceneComponent.K2_AddRelativeLocation` _array_element (`KismetMathLibrary.MakeVector` (* _returnvalue_2 (`self.Area`)) (* (`self.plus`) (`self.Area`))) false false)
      (if (and (== _returnvalue_2 0) (> _array_index 0))
        (bind _result (`/Engine/EditorBlueprintResources/StandardMacros.IncrementInt` (`self.plus`))
          (:`  `
            (set `self.plus` _result))))))
  (for _array_element_2 (`self.Niagara`)
    (if (`KismetSystemLibrary.IsValid` _array_element_2)
      (`SceneComponent.K2_AddRelativeLocation` _array_element_2 (`KismetMathLibrary.MakeVector` (* (* (- (`KismetMathLibrary.FTrunc` (`KismetMathLibrary.Abs` _x_2)) 1) _area) -0.5) (* (* (- (`KismetMathLibrary.FTrunc` (`KismetMathLibrary.Abs` _y_2)) 1) _area) -0.5)) false false)))
  (for _array_element_3 (`self.Niagara`)
    (bind _output_get (set `self.rain` _array_element_3))
    (if (`KismetSystemLibrary.IsValid` _output_get)
      (`|ExecutionSequence`
        (:`then_0`
          (if (`|EnumEquality` _rain_type "NewEnumerator1")
            (set `self.intensity` 0.5)
            (set `self.Min_Length` 0.2)
            (set `self.Max_Length` 0.5)
            (set `self.Min_Width` 0.4)
            (set `self.Max_Width` 0.5)
            (set `self.Spawn_Rate` 200)
            (set `self.Max_rot` 1.0)
            (set `self.Min_rot` -1.0)
            (set `self.velocity` 900.0)
            (set `self.Hit_Type` 1)
            (set `self.Hit_Scale` 1.0)
            (set `self.Area` 1000.0 :!label _label)
            (set `self.HitBrightness` 0.5)
            (`NiagaraComponent.SetVariableFloat` _rain_2 "int" (`self.intensity`) :!label _label_2)
            (`NiagaraComponent.SetVariableVec3` _rain_2 "color" (`KismetMathLibrary.MakeVector` _r _g _b))
            (`NiagaraComponent.SetVariableFloat` _rain_3 "switch" (`KismetMathLibrary.Conv_IntToDouble` (`self.Hit_Type`)))
            (`NiagaraComponent.SetVariableFloat` _rain_3 "Rain_Intensity" (`KismetMathLibrary.Conv_IntToDouble` (`self.Spawn_Rate`)))
            (`NiagaraComponent.SetVariableFloat` _rain_4 "lemin" (`KismetMathLibrary.MapRangeClamped` (`self.Min_Length`) 0.0 1.0 1.0 -1.0))
            (`NiagaraComponent.SetVariableFloat` _rain_4 "lemax" (`KismetMathLibrary.MapRangeClamped` (`self.Max_Length`) 0.0 1.0 1.0 -1.0))
            (`NiagaraComponent.SetVariableFloat` _rain_4 "wgmin" (`self.Min_Width`))
            (`NiagaraComponent.SetVariableFloat` _rain_4 "wgmax" (`self.Max_Width`))
            (`NiagaraComponent.SetVariableFloat` _rain_5 "max_Rot" (`self.Max_rot`))
            (`NiagaraComponent.SetVariableFloat` _rain_5 "min_Rot" (`self.Min_rot`))
            (`NiagaraComponent.SetVariableFloat` _rain "vel" _velocity)
            (`NiagaraComponent.SetVariableFloat` _rain "life" (`KismetMathLibrary.MapRangeClamped` _velocity 100.0 1000.0 5.0 2.0))
            (`NiagaraComponent.SetVariableFloat` _rain_6 "hitdropscale" (`self.Hit_Scale`))
            (`NiagaraComponent.SetVariableFloat` _rain_6 "Area" (`self.Area`))
            (`NiagaraComponent.SetVariableFloat` _rain_6 "alpha" (`self.HitBrightness`))))
        (:`then_1`
          (if (`|EnumEquality` _rain_type "NewEnumerator2")
            (set `self.intensity` 0.7)
            (set `self.Min_Length` 0.5)
            (set `self.Max_Length` 1.0)
            (set `self.Min_Width` 0.35)
            (set `self.Max_Width` 0.45)
            (set `self.Spawn_Rate` 600)
            (set `self.Max_rot` 5.0)
            (set `self.Min_rot` -5.0)
            (set `self.velocity` 1000.0)
            (set `self.Hit_Type` 2)
            (set `self.Hit_Scale` 0.6)
            (goto _label)))
        (:`then_2`
          (if (`|EnumEquality` _rain_type "NewEnumerator3")
            (set `self.intensity` 1.0)
            (set `self.Min_Length` 0.2)
            (set `self.Max_Length` 1.0)
            (set `self.Min_Width` 0.4)
            (set `self.Max_Width` 0.5)
            (set `self.Spawn_Rate` 1000)
            (set `self.Max_rot` 10.0)
            (set `self.Min_rot` -10.0)
            (set `self.velocity` 1200.0)
            (set `self.Hit_Type` 3)
            (set `self.Hit_Scale` 0.6)
            (goto _label)))
        (:`then_3`
          (if (`|EnumEquality` _rain_type "NewEnumerator4")
            (set `self.Area` 2500.0)
            (set `self.intensity` 0.2)
            (set `self.Min_Length` 0.2)
            (set `self.Max_Length` 1.0)
            (set `self.Min_Width` 0.4)
            (set `self.Max_Width` 0.5)
            (set `self.Spawn_Rate` 18000)
            (set `self.Max_rot` 10.0)
            (set `self.Min_rot` -10.0)
            (set `self.velocity` 1200.0)
            (set `self.Hit_Type` 3)
            (set `self.Hit_Scale` 0.6)
            (set `self.Color` (struct :`R` 0.341667 :`G` 0.341667 :`B` 0.341667 :`A` 1.0))
            (goto _label)))
        (:`then_4`
          (if (`|EnumEquality` _rain_type "NewEnumerator0")
            (goto _label_2)))))))

(fn `TurnAlarmOn`
  (params (AlarmActivated :type Boolean))
  (if AlarmActivated
    (`self.BeginAlarm`)))

(fn `UserConstructionScript`
  (`self.InitPlay`))