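; Rain FX actor that runs a water particle effect along an editable spline.
; The construction script passes the spline, spawn count, trail length, size range and speed into the Niagara component SplineParticle.
; A Type enum selects one of five material pairs, then applies the shared upward fade and hit brightness settings.
; All setup happens at construction, with no active event graph logic.
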(fn `UserConstructionScript`
  (bind _spline_particle (`self.Spline_Particle`))
  (bind _type (`self.Type`))
  (bind _spline_particle_2 (`self.Spline_Particle`))
  (bind _spline_particle_3 (`self.Spline_Particle`))
  (bind (_x _y) (`KismetMathLibrary.BreakVector2D` (`self.Min/Max(Size)`)))
  (`NiagaraComponent.SetVariableObject` _spline_particle "spline" (`self.Spline`))
  (`NiagaraComponent.SetVariableInt` _spline_particle "spawn" (`self.Spawn_Count`))
  (`NiagaraComponent.SetVariableInt` _spline_particle "trail" (`self.Trail_Length`))
  (`NiagaraComponent.SetVariableFloat` _spline_particle "scmin" _x)
  (`NiagaraComponent.SetVariableFloat` _spline_particle "scmax" _y)
  (`NiagaraComponent.SetVariableFloat` (`self.Spline_Particle`) "speed" (`self.Speed`))
  (`|ExecutionSequence`
    (:`then_0`
      (if (`|EnumEquality` _type "NewEnumerator0")
        (`NiagaraComponent.SetVariableMaterial` _spline_particle_3 "Mat" "/Game/Assets/Rain_FX/RainFX_Tools/Material/Master/M_SW_s_A_H.M_SW_s_A_H")
        (`NiagaraComponent.SetVariableMaterial` _spline_particle_3 "Mat2" "/Game/Assets/Rain_FX/RainFX_Tools/Material/Master/M_SW_m_A_H.M_SW_m_A_H")
        (`NiagaraComponent.SetVariableFloat` _spline_particle_3 "UpFade" (`self.Up_Fade`) :!label _label)
        (`NiagaraComponent.SetVariableFloat` _spline_particle_3 "Alpha" (`self.HitBrightness`))))
    (:`then_1`
      (if (`|EnumEquality` _type "NewEnumerator1")
        (`NiagaraComponent.SetVariableMaterial` _spline_particle_3 "Mat" "/Game/Assets/Rain_FX/RainFX_Tools/Material/Master/M_SW_s_B_H.M_SW_s_B_H")
        (`NiagaraComponent.SetVariableMaterial` _spline_particle_3 "Mat2" "/Game/Assets/Rain_FX/RainFX_Tools/Material/Master/M_SW_m_B_H.M_SW_m_B_H")
        (goto _label)))
    (:`then_2`
      (if (`|EnumEquality` _type "NewEnumerator2")
        (`NiagaraComponent.SetVariableMaterial` _spline_particle_2 "Mat" "/Game/Assets/Rain_FX/RainFX_Tools/Material/Master/M_SW_s_C_H.M_SW_s_C_H")
        (`NiagaraComponent.SetVariableMaterial` _spline_particle_2 "Mat2" "/Game/Assets/Rain_FX/RainFX_Tools/Material/Master/M_SW_m_C_H.M_SW_m_C_H")
        (goto _label)))
    (:`then_3`
      (if (`|EnumEquality` _type "NewEnumerator3")
        (`NiagaraComponent.SetVariableMaterial` _spline_particle_2 "Mat" "/Game/Assets/Rain_FX/RainFX_Tools/Material/Master/M_SW_s_D_H.M_SW_s_D_H")
        (`NiagaraComponent.SetVariableMaterial` _spline_particle_2 "Mat2" "/Game/Assets/Rain_FX/RainFX_Tools/Material/Master/M_SW_m_D_H.M_SW_m_D_H")
        (goto _label)))
    (:`then_4`
      (if (`|EnumEquality` _type "NewEnumerator4")
        (`NiagaraComponent.SetVariableMaterial` _spline_particle_2 "Mat" "/Game/Assets/Rain_FX/RainFX_Tools/Material/Master/M_SW_s_E_H.M_SW_s_E_H")
        (`NiagaraComponent.SetVariableMaterial` _spline_particle_2 "Mat2" "/Game/Assets/Rain_FX/RainFX_Tools/Material/Master/M_SW_m_E_H.M_SW_m_E_H")
        (goto _label)))))