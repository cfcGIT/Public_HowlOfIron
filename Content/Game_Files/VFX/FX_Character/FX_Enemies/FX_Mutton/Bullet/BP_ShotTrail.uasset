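; BP_ShotTrail is a bullet trail effect actor, filed under the Mutton enemy's VFX, that travels to a target location.
; On BeginPlay it applies a Scale variable to its Scene component.
; Each tick it moves its Sphere at constant ProjectileSpeed toward TargetLocation without sweeping, then destroys the actor once the Sphere arrives within a small tolerance.
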(event `self.ReceiveBeginPlay`
  (`SceneComponent.SetRelativeScale3D` (`self.Scene`) (`self.Scale`)))

(event `self.ReceiveTick`
  (params (DeltaSeconds :type "Float (single-precision)"))
  (bind _sphere (`self.Sphere`))
  (`SceneComponent.K2_SetWorldLocation` _sphere (`KismetMathLibrary.VInterpTo_Constant` (`SceneComponent.K2_GetComponentLocation` (`self.Sphere`)) (`self.TargetLocation`) (`GameplayStatics.GetWorldDeltaSeconds`) (`self.ProjectileSpeed`)) false false)
  (if (== (`SceneComponent.K2_GetComponentLocation` _sphere) (`self.TargetLocation`) :`ErrorTolerance` 1.0)
    (`self.K2_DestroyActor`)))

(fn `UserConstructionScript`)