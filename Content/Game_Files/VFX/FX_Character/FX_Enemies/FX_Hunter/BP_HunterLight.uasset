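; BP_HunterLight is a VFX actor that follows a Hunter enemy and yaws toward the werewolf, driving a hunter light's visibility.
; Each Tick, unless the Hunter is Disabled, it updates its transform and checks the combat tag.
; After a sustained out-of-combat delay, it raises OpacityHunterLight in the MPC_HIClaws parameter collection as Hunter-to-werewolf distance grows.
; Entering combat resets the timer and zeroes that opacity.
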(event `self.ReceiveBeginPlay`
  (set `self.MPC` "/Game/Game_Files/VFX/FX_Character/FX_Werewolf/FX/MPC_HIClaws.MPC_HIClaws"))

(event `self.ReceiveTick`
  (params (DeltaSeconds :type "Float (single-precision)"))
  (bind _timer (`self.timer`))
  (bind (_returnvalue_x _returnvalue_y) (`KismetMathLibrary.BreakVector` (`self.K2_GetActorLocation` self)))
  (bind (_returnvalue_x_2 _returnvalue_y_2 _returnvalue_z) (`KismetMathLibrary.BreakVector` (`self.K2_GetActorLocation` (`self.hunter`))))
  (if (`GameplayTagAssetInterface.HasMatchingGameplayTag` (`AbilitySystemBlueprintLibrary.GetAbilitySystemComponent` (`self.hunter`)) (struct :`TagName` "Character.State.Disabled"))
    _
    (elif (`KismetSystemLibrary.IsValid` (`self.hunter`))
      (`self.K2_SetActorLocation` (`KismetMathLibrary.MakeVector` _returnvalue_x_2 _returnvalue_y_2 _returnvalue_z) false true)
      (bind _returnvalue (`HIGameData.HIGetWerewolfLocation`))
      (`self.K2_SetActorRotation` (`KismetMathLibrary.Conv_VectorToRotator` (- (`KismetMathLibrary.MakeVector` (.x _returnvalue) (.y _returnvalue)) (`KismetMathLibrary.MakeVector` _returnvalue_x _returnvalue_y))))
      (bind _returnvalue_2 (message `GameplayTagAssetInterface.HasMatchingGameplayTag` (`HIAbilityCharacter.abilitySystem` (`self.hunter`)) (struct :`TagName` "Enemy.Ability.Combat")))
      (if _returnvalue_2
        (set `self.timer` 0.0)
        (if (`self.activeray`)
          (`KismetMaterialLibrary.SetScalarParameterValue` (`self.MPC`) "OpacityHunterLight")
          (set `self.activeray` false))
        (elif (> _timer 30.0)
          (if (not (`self.activeray`))
            (set `self.activeray` true))
          (bind _returnvalue_3 (`HIGameData.HIGetWerewolfLocation`))
          (`KismetMaterialLibrary.SetScalarParameterValue` (`self.MPC`) "OpacityHunterLight" (`KismetMathLibrary.MapRangeClamped` (+ (`KismetMathLibrary.Vector_Distance` (`self.K2_GetActorLocation` (`self.hunter`)) _returnvalue_3) -2000.0) 0.0 2000.0 0.0 0.2))
          (else
            (set `self.timer` (+ _timer DeltaSeconds))))))))

(fn `UserConstructionScript`)