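; BP_ElectricPole is an electric pole prop that strings four cables to linked poles in the level.
; Its construction script converts world locations of the linked poles' sphere components into local space and sets them as cable end locations.
; Cables 1–2 attach to NextElectricalPole and 3–4 to NextElectricalPole1, though only the former is validity-checked.
; The ResetWire branch is empty, and no runtime logic exists.
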(fn `UserConstructionScript`
  (if (`self.ResetWire`)
    _
    (else
      _))
  (`/Engine/EditorBlueprintResources/StandardMacros.IsValid` (`self.NextElectricalPole`)
    (:`Is Valid`
      (set `CableComponent.EndLocation` (`KismetMathLibrary.InverseTransformLocation` (`self.GetTransform`) (`SceneComponent.K2_GetComponentLocation` (`/Game/Game_Files/Enviorment/Props/ElectricPole/Meshes/BP_ElectricPole.Sphere1` (`self.NextElectricalPole`)))) (`self.Cable1`))
      (set `CableComponent.EndLocation` (`KismetMathLibrary.InverseTransformLocation` (`self.GetTransform`) (`SceneComponent.K2_GetComponentLocation` (`/Game/Game_Files/Enviorment/Props/ElectricPole/Meshes/BP_ElectricPole.Sphere2` (`self.NextElectricalPole`)))) (`self.Cable2`))
      (set `CableComponent.EndLocation` (`KismetMathLibrary.InverseTransformLocation` (`self.GetTransform`) (`SceneComponent.K2_GetComponentLocation` (`/Game/Game_Files/Enviorment/Props/ElectricPole/Meshes/BP_ElectricPole.Sphere3` (`self.NextElectricalPole_1`)))) (`self.Cable3`))
      (set `CableComponent.EndLocation` (`KismetMathLibrary.InverseTransformLocation` (`self.GetTransform`) (`SceneComponent.K2_GetComponentLocation` (`/Game/Game_Files/Enviorment/Props/ElectricPole/Meshes/BP_ElectricPole.Sphere4` (`self.NextElectricalPole_1`)))) (`self.Cable4`)))))