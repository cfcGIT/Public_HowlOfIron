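; BP_Streetlight is a streetlight prop Blueprint with a StacionaryCenter component.
; Its only logic is unconnected and never runs: a distance cull comparing squared distance from the werewolf's location to the streetlight against a 6000-unit radius.
; That graph would turn StacionaryCenter's visibility and shadow casting off beyond the radius and on within it.
; The construction script is empty.
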(fn `UserConstructionScript`)