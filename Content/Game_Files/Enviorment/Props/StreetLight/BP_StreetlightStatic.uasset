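; BP_StreetlightStatic is a streetlight prop that the player werewolf can dash through.
; A detection capsule enables actor tick only while the werewolf overlaps it.
; Each tick checks the werewolf's ability system for the Dash gameplay tag, and when present disables the blocking capsule's collision, restoring query and physics collision after a half-second delay.
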(event `self.CapsuleDetect.OnComponentBeginOverlap`
  (params (OverlappedComponent :type "PrimitiveComponent Object Reference") (OtherActor :type "Actor Object Reference") (OtherComp :type "PrimitiveComponent Object Reference") (OtherBodyIndex :type Integer) (bFromSweep :type Boolean) (SweepResult :type "HitResult Structure (by ref)"))
  (bind _returnvalue (`HIGameData.HIGetPlayerWerewolf`))
  (if (== _returnvalue OtherActor)
    (`self.SetActorTickEnabled` true)))

(event `self.CapsuleDetect.OnComponentEndOverlap`
  (params (OverlappedComponent :type "PrimitiveComponent Object Reference") (OtherActor :type "Actor Object Reference") (OtherComp :type "PrimitiveComponent Object Reference") (OtherBodyIndex :type Integer))
  (bind _returnvalue (`HIGameData.HIGetPlayerWerewolf`))
  (if (== _returnvalue OtherActor)
    (`self.SetActorTickEnabled` false)))

(event `self.ReceiveTick`
  (params (DeltaSeconds :type "Float (single-precision)"))
  (bind _returnvalue (`HIGameData.HIGetPlayerWerewolf`))
  (bind _returnvalue_2 (message `GameplayTagAssetInterface.HasMatchingGameplayTag` (`HIAbilityCharacter.abilitySystem` _returnvalue) (struct :`TagName` "Werewolf.Ability.Dash")))
  (if _returnvalue_2
    (`PrimitiveComponent.SetCollisionEnabled` (`self.Capsule`) "NoCollision")
    (`KismetSystemLibrary.Delay` 0.5)
    (`PrimitiveComponent.SetCollisionEnabled` (`self.Capsule`) "QueryAndPhysics")))

(fn `UserConstructionScript`)