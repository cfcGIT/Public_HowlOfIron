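; Light bulb prop with a spotlight that can flicker and sweep back and forth, each behavior toggled by its own flag.
; Flicker uses a self-restarting random timer that zeroes intensity for a random off time, then restores it.
; Rotation squares the base to world zero, then a looping timer drives a timeline forward or in reverse, lerping arm yaw and body pitch.
; The direction flips after a stop delay when the timeline finishes.
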(event `ResetTimer`
  (bind (_flickertimerange_x _flickertimerange_y) (`KismetMathLibrary.BreakVector2D` (`self.FlickerTimeRange`)))
  ;[1 1 1] Flickering
  (`KismetSystemLibrary.K2_SetTimerDelegate` (delegate `LightFlicker`) (`KismetMathLibrary.RandomFloatInRange` _flickertimerange_x _flickertimerange_y) :!label _label))

(event `self.ReceiveBeginPlay`
  (`|ExecutionSequence`
    (:`then_0`
      ;[1 1 1] Flickering
      (if (`self.isFlickering`)
        (goto _label)))
    (:`then_1`
      ;[1 1 1] Rotation
      (if (`self.Is Rotating`)
        (`self.Reset Rotation`)
        (`KismetSystemLibrary.K2_SetTimerDelegate` (delegate `RotateLight`) 0.5 true)))))

(event `LightFlicker`
  ;[1 1 1] Flickering
  (`self.SimpleFlick`))

(event `SimpleFlick`
  (bind _spotlight (`self.SpotLight`))
  (bind (_offtimeflicker_x _offtimeflicker_y) (`KismetMathLibrary.BreakVector2D` (`self.offTimeFlicker`)))
  ;[1 1 1] Flickering
  ;;[0.04314 0.04314 0.04314] Simple Flicker ON/OFF
  (set `self.IntensityBackup` (`LightComponentBase.Intensity` _spotlight))
  (`LightComponent.SetIntensity` _spotlight 0.0)
  (`KismetSystemLibrary.Delay` (`KismetMathLibrary.RandomFloatInRange` _offtimeflicker_x _offtimeflicker_y))
  (`LightComponent.SetIntensity` _spotlight (`self.IntensityBackup`))
  (`self.ResetTimer`))

(event `RotateLight`
  (bind (_rotation_range_a_roll _rotation_range_a_pitch _rotation_range_a_yaw) (`KismetMathLibrary.BreakRotator` (`self.Rotation Range A`)))
  (bind (_rotation_range_b_roll _rotation_range_b_pitch _rotation_range_b_yaw) (`KismetMathLibrary.BreakRotator` (`self.Rotation Range B`)))
  ;[1 1 1] Rotation
  ;;[0.04688 0.04688 0.04688] Rotate Light
  (if (`self.Right Rotation_0`)
    (bind (_direction _z) (`Timeline|Timeline_0` :!label _label_2)
      (:`Update`
        (`SceneComponent.K2_SetWorldRotation` (`self.SM_LightBulbArm`) (`KismetMathLibrary.RLerp` (`KismetMathLibrary.MakeRotator` 0.0 0.0 _rotation_range_a_yaw) (`KismetMathLibrary.MakeRotator` 0.0 0.0 _rotation_range_b_yaw) _z) false false)
        (`SceneComponent.K2_SetRelativeRotation` (`self.SM_LightBulbBody`) (`KismetMathLibrary.RLerp` (`KismetMathLibrary.MakeRotator` 0.0 _rotation_range_a_pitch) (`KismetMathLibrary.MakeRotator` 0.0 _rotation_range_b_pitch) _z) false false))
      (:`Finished`
        (`KismetSystemLibrary.Delay` (`self.Stop Time`))
        (set `self.Right Rotation_0` (not (`self.Right Rotation_0`)))))
    (else
      (goto _label_2 :!via `Reverse`))))

(event `Reset Rotation`
  ;[1 1 1] Set base to be 0,0,0 rotation
  (`SceneComponent.K2_SetWorldRotation` :`self` (`self.SM_LightBulbBase`)))

(fn `UserConstructionScript`)