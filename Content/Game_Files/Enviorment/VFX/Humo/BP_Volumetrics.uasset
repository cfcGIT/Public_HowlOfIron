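; BP_Volumetrics is a smoke VFX actor that fakes a volume by stacking mesh slices upward at runtime.
; On BeginPlay it adds static mesh components at even Z steps derived from VolumenHeight and Volumenresolution.
; The base Plane and each slice get dynamic materials fed their world Z and the volume height.
; The parameter names differ: the Plane's use underscores (MinFrom_BP), the slices' use spaces (MinFrom BP).
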(event `self.ReceiveBeginPlay`
  (bind _plane (`self.Plane`))
  (bind (_returnvalue_x _returnvalue_y _returnvalue_z) (`KismetMathLibrary.BreakVector` (`SceneComponent.K2_GetComponentLocation` _plane)))
  (bind _returnvalue (+ (`self.Pre-Volumen-Height`) (/ (`self.Volumen-Height`) (`KismetMathLibrary.Conv_IntToDouble` (`self.Volumen-resolution`)))))
  (bind _returnvalue_2 (`PrimitiveComponent.CreateDynamicMaterialInstance` _plane 0 (`PrimitiveComponent.GetMaterial` (`self.Plane`) 0) "None"))
  (`MaterialInstanceDynamic.SetScalarParameterValue` _returnvalue_2 "MinFrom_BP" _returnvalue_z)
  (`MaterialInstanceDynamic.SetScalarParameterValue` _returnvalue_2 "MaxFrom_BP" (`self.Volumen-Height`))
  (for _ (range (+ (`self.Volumen-resolution`) 1))
    (bind _returnvalue_3 (`AddComponent|NODE_AddStaticMeshComponent-0` :`RelativeTransform` (`KismetMathLibrary.MakeTransform` (`KismetMathLibrary.MakeVector` 0.0 0.0 _returnvalue))))
    (set `self.Pre-Volumen-Height` _returnvalue)
    (bind _returnvalue_4 (`PrimitiveComponent.CreateDynamicMaterialInstance` _returnvalue_3 0 (`PrimitiveComponent.GetMaterial` _returnvalue_3 0) "None"))
    (bind (_returnvalue_x_2 _returnvalue_y_2 _returnvalue_z_2) (`KismetMathLibrary.BreakVector` (`SceneComponent.K2_GetComponentLocation` _returnvalue_3)))
    (`MaterialInstanceDynamic.SetScalarParameterValue` _returnvalue_4 "MinFrom BP" _returnvalue_z_2)
    (`MaterialInstanceDynamic.SetScalarParameterValue` _returnvalue_4 "MaxFrom BP" (`self.Volumen-Height`))))

(fn `UserConstructionScript`)