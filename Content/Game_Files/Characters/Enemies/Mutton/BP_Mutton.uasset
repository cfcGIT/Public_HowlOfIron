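; BP_Mutton is the Blueprint for the Mutton enemy, exposing world-space attachment points on its current weapon.
; Two getters read sockets on the ActualWeapon's AccessoryMesh: the muzzle transform uses the weapon's own ShootSocketName, while the hand transform uses a fixed LeftHand socket.
; The construction script is empty, and the file defines no other behavior.
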(fn `Get Muzzle Socket Transform`
  (returns (Transform :type "Transform Structure"))
  (bind _actualweapon (`self.actualWeapon`))
  (return (`SceneComponent.GetSocketTransform` (`HIEnemyAccessory.accessoryMesh` _actualweapon) (`HIEnemyAccessory.shootSocketName` _actualweapon) "RTS_World")))

(fn `GetHandSocketTransform`
  (returns (Transform :type "Transform Structure"))
  (return (`SceneComponent.GetSocketTransform` (`HIEnemyAccessory.accessoryMesh` (`self.actualWeapon`)) "LeftHand" "RTS_World")))

(fn `UserConstructionScript`)