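; Green Mutton enemy Blueprint that plays an absorption effect toward the werewolf when it dies.
; The death event spawns a Niagara absorption system at the actor's location and starts a short timed window.
; During that window, Tick feeds the werewolf's front attack socket position into the system's HitPosition variable, so the effect tracks the moving werewolf.
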(event `self.ReceiveTick`
  (params (DeltaSeconds :type "Float (single-precision)"))
  (if (`self.smoking`)
    (bind _output_get (set `self.smokeActivatedTimer` (+ DeltaSeconds (`self.smokeActivatedTimer`))))
    (if (< _output_get 3.0)
      (`NiagaraComponent.SetVariableVec3` (stale `self.HIGreenDeath` _returnvalue) "HitPosition" (`SceneComponent.GetSocketLocation` (`Character.Mesh` (`self.HIGetWerewolf`)) "FrontAttackSocket") :!label _label)
      (else
        (set `self.smoking` false)))))

(event `self.HIGreenDeath`
  (set `self.smoking` true)
  (bind _returnvalue (`NiagaraFunctionLibrary.SpawnSystemAtLocation` "/Game/Game_Files/VFX/FX_Character/FX_Enemies/FX_Mutton/GreenMuttonExplosion/NS_GreenMuttonAbsorbtion.NS_GreenMuttonAbsorbtion" (`self.K2_GetActorLocation`)))
  (goto _label))

(fn `UserConstructionScript`
  (`parent.UserConstructionScript`))