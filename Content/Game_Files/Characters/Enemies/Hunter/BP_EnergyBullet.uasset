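; Enemy energy bullet, filed under Hunter, that turns every tick to face the player werewolf.
; It enables collision shortly after BeginPlay and returns to the object pooler on a lifetime timer.
; Overlaps with enemies and their accessories are ignored.
; Any other overlap despawns it, first applying its gameplay effect spec through the source ability system if the target has an ability system component.
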(event `self.ReceiveBeginPlay`
  (`KismetSystemLibrary.K2_SetTimerDelegate` (delegate `DestroyDelay`) 15.0)
  (`self.SetActorEnableCollision` false)
  (`KismetSystemLibrary.Delay` 0.2)
  (`self.SetActorEnableCollision` true))

(event `DestroyDelay`
  (`HIObjectPooler_Actors.DespawnItem` (`HIObjectPooler_Actors.HIGetObjectPooler` null) self))

(event `self.ReceiveActorBeginOverlap`
  (params (OtherActor :type "Actor Object Reference"))
  (bind _abilitysystemsource (`self.AbilitySystemSource`))
  (bind _returnvalue (`AbilitySystemBlueprintLibrary.GetAbilitySystemComponent` (cast `HIAbilityCharacter` OtherActor :!pure true)))
  (cast `HIEnemy` OtherActor
    (:`CastFailed`
      (cast `HIEnemyAccessory` OtherActor
        (:`CastFailed`
          (if (and (`KismetSystemLibrary.IsValid` _abilitysystemsource) (`KismetSystemLibrary.IsValid` _returnvalue))
            (`AbilitySystemComponent.BP_ApplyGameplayEffectSpecToTarget` _abilitysystemsource (`self.GameplayEffectSpec`) _returnvalue))
          (`HIObjectPooler_Actors.DespawnItem` (`HIObjectPooler_Actors.HIGetObjectPooler` null) self))))))

(event `self.ReceiveTick`
  (params (DeltaSeconds :type "Float (single-precision)"))
  (bind _returnvalue (`HIGameData.HIGetPlayerWerewolf`))
  (`self.K2_SetActorRotation` (`KismetMathLibrary.FindLookAtRotation` (`self.K2_GetActorLocation`) (`self.K2_GetActorLocation` _returnvalue))))

(fn `UserConstructionScript`)