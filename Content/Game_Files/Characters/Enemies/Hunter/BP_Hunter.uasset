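; Hunter boss enemy with a screen boss HUD, a material-driven shield and a cutscene death.
; The overhead EnemyBars widget is hidden but remains the data source, polled each Tick to debug-print and feed health and vulnerability to the HUD.
; KillBoss plays the FinalExecution cutscene with Vincent Volk and collapses the HUD.
; ShowEnd plays the end-of-demo UI, but its cutscene-finish binding never runs; GetHandSocketTransform is an empty stub.
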(event `self.ReceiveBeginPlay`
  (`SceneComponent.SetVisibility` (`self.enemyBars`) false false)
  (`SceneComponent.SetHiddenInGame` (`self.enemyBars`) true false)
  (bind _returnvalue (`|CreateWidget` "/Game/Game_Files/UI/EnemiesHUD/UI_BossHUD.UI_BossHUD_C"))
  (bind _output_get (set `self.BossHUD` _returnvalue))
  (`UserWidget.AddToViewport` _output_get -1)
  (`Widget.SetVisibility` _output_get "Hidden"))

(event `Event KillBoss`
  (bind _outactors (`GameplayStatics.GetAllActorsOfClassWithTag` "/Game/Logic/LevelDesign_Utilities/CutscenesUtilities/BP_CutscenesTrigger.BP_CutscenesTrigger_C" "FinalExecution"))
  (bind _asbp_vincent_volk (cast `/Game/Game_Files/Characters/Vincent_Volk/BP_Vincent_Volk` (`self.HIGetWerewolf`)))
  (`/Game/Logic/LevelDesign_Utilities/CutscenesUtilities/BP_CutscenesTrigger.Event PlayCutscene` (`|GetArrayItem` _outactors) _asbp_vincent_volk)
  (`Widget.SetVisibility` (`self.BossHUD`) "Collapsed"))

(event `self.ReceiveTick`
  (params (DeltaSeconds :type "Float (single-precision)"))
  (bind _ashiboss_hud (cast `HIBossHUD` (`WidgetComponent.GetWidget` (`self.enemyBars`))))
  (bind _returnvalue (`HIBossHUD.HIGetvulnerability` _ashiboss_hud))
  (`KismetSystemLibrary.PrintString` (`KismetStringLibrary.Conv_BoolToString` _returnvalue) true true (struct :`G` 0.66 :`B` 1.0 :`A` 1.0) 0.0)
  (bind _returnvalue_2 (/ (`HIEnemyHUD.health` _ashiboss_hud) (`HIEnemyHUD.maxHealth` _ashiboss_hud)))
  (`KismetSystemLibrary.PrintString` (`KismetStringLibrary.Conv_DoubleToString` _returnvalue_2) true true (struct :`G` 0.66 :`B` 1.0 :`A` 1.0) 0.0)
  (`/Game/Game_Files/UI/EnemiesHUD/UI_BossHUD.Event Update` (`self.BossHUD`) _returnvalue_2 _returnvalue))

(event `ActivateShield`
  (`MeshComponent.SetScalarParameterValueOnMaterials` (`self.Shield`) "Shield" 1.0))

(event `Event ShowEnd`
  (bind _returnvalue (`HIGameData.HIGetPlayerWerewolf`))
  (bind _asbp_vincent_volk (cast `/Game/Game_Files/Characters/Vincent_Volk/BP_Vincent_Volk` _returnvalue))
  (bind _asui_vincent_hud (cast `/Game/Game_Files/UI/VincentHUD/UI_VincentHUD` (`HIWerewolf.widgetref` _asbp_vincent_volk)))
  (`/Game/Game_Files/UI/VincentHUD/UI_VincentHUD.Event PlayEndDemo` _asui_vincent_hud))

(event `DisableShield`
  (`MeshComponent.SetScalarParameterValueOnMaterials` (`self.Shield`) "Shield" 0.0))

(fn `Get Muzzle Socket Transform`
  (returns (Transform :type "Transform Structure"))
  (bind _actualweapon (`self.actualWeapon`))
  (return (`SceneComponent.GetSocketTransform` (`HIEnemyAccessory.accessoryMesh` _actualweapon) (`HIEnemyAccessory.shootSocketName` _actualweapon) "RTS_World")))

(fn `GetHandSocketTransform`
  (returns (Transform :type "Transform Structure"))
  (return))

(fn `ShowHUD`
  (`Widget.SetVisibility` (`self.BossHUD`) "HitTestInvisible"))

(fn `UserConstructionScript`)