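; Player controller for Vincent Volk that handles cutscene skipping, input-device detection and a secret katana cheat.
; While skipping is allowed, Tick feeds the B or gamepad right face button hold time to the HUD and swaps its prompt icon.
; WASD and left-stick input set the controller type on the game instance.
; A Konami-code state machine advances SecretSkinStep from keyboard or gamepad presses, calling SwitchKatana on the werewolf when completed.
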(event `self.ReceiveTick`
  (params (DeltaSeconds :type "Float (single-precision)"))
  (bind _returnvalue (`self.GetInputKeyTimeDown` "Gamepad_FaceButton_Right"))
  (bind _returnvalue_2 (`self.GetInputKeyTimeDown` "B"))
  (if (`self.CanSkip`)
    (bind _ashiwerewolf (cast `HIWerewolf` (`GameplayStatics.GetPlayerCharacter` 0)))
    (bind _asui_vincent_hud (cast `/Game/Game_Files/UI/VincentHUD/UI_VincentHUD` (`HIWerewolf.widgetref` _ashiwerewolf)))
    (if (`/Game/Game_Files/UI/VincentHUD/UI_VincentHUD.IsPlayingCutscene` _asui_vincent_hud)
      (`/Engine/EditorBlueprintResources/StandardMacros.IsValid` (`/Game/Game_Files/UI/VincentHUD/UI_VincentHUD.CutscenePlayer` _asui_vincent_hud)
        (:`Is Valid`
          (if (> _returnvalue_2 0.0)
            (set `/Game/Game_Files/UI/VincentHUD/UI_VincentHUD.TimeToSkip` _returnvalue_2 _asui_vincent_hud)
            (bind _image_79 (`/Game/Game_Files/UI/VincentHUD/UI_VincentHUD.Image_79` _asui_vincent_hud))
            (`Image.SetBrushFromTexture` _image_79 "/Game/Assets/Zombie_Game_UI_Elements/PC_Icons/B.B" false)
            (`Widget.SetRenderScale` _image_79 (0.65 0.65))
            (elif (> _returnvalue 0.0)
              (set `/Game/Game_Files/UI/VincentHUD/UI_VincentHUD.TimeToSkip` _returnvalue _asui_vincent_hud)
              (bind _image_79_2 (`/Game/Game_Files/UI/VincentHUD/UI_VincentHUD.Image_79` _asui_vincent_hud))
              (`Image.SetBrushFromTexture` _image_79_2 "/Game/Assets/Zombie_Game_UI_Elements/Console_Icons/XB.XB" false)
              (`Widget.SetRenderScale` _image_79_2 (1.0 1.0))
              (else
                (set `/Game/Game_Files/UI/VincentHUD/UI_VincentHUD.TimeToSkip` 0.0 _asui_vincent_hud)))))
        (:`Is Not Valid`
          (set `/Game/Game_Files/UI/VincentHUD/UI_VincentHUD.TimeToSkip` 0.0 _asui_vincent_hud))))))

(event `InputAxisKey|Gamepad_LeftY`
  (params (AxisValue :type "Float (single-precision)"))
  (if (!= AxisValue 0.0)
    (bind _returnvalue (`HIGameData.HIGetGameInstance`))
    (bind _asbp_higame_instance (cast `/Game/Logic/Scripts/Game/BP_HIGameInstance` _returnvalue))
    (`/Game/Logic/Scripts/Game/BP_HIGameInstance.SetControllerType` _asbp_higame_instance "NewEnumerator1")))

(event `InputAxisKey|Gamepad_LeftX`
  (params (AxisValue :type "Float (single-precision)"))
  (if (!= AxisValue 0.0)
    (bind _returnvalue (`HIGameData.HIGetGameInstance`))
    (bind _asbp_higame_instance (cast `/Game/Logic/Scripts/Game/BP_HIGameInstance` _returnvalue))
    (`/Game/Logic/Scripts/Game/BP_HIGameInstance.SetControllerType` _asbp_higame_instance "NewEnumerator1")))

(event `Key|W`
  (params (Key :type "Key Structure"))
  (:`Pressed`
    (bind _returnvalue (`HIGameData.HIGetGameInstance` :!label _label))
    (bind _asbp_higame_instance (cast `/Game/Logic/Scripts/Game/BP_HIGameInstance` _returnvalue))
    (`/Game/Logic/Scripts/Game/BP_HIGameInstance.SetControllerType` _asbp_higame_instance "NewEnumerator0")))

(event `Key|S`
  (params (Key :type "Key Structure"))
  (:`Pressed`
    (goto _label)))

(event `Key|A`
  (params (Key :type "Key Structure"))
  (:`Pressed`
    (goto _label)))

(event `Key|D`
  (params (Key :type "Key Structure"))
  (:`Pressed`
    (goto _label)))

(event `Key|Gamepad_DPad_Up`
  (params (Key :type "Key Structure"))
  (:`Pressed`
    (`self.SetCurrentSkinStep` (select `/Game/Logic/Enumerators/E_SecretSkinSteps` (`self.SecretSkinStep`) :`NewEnumerator12` "NewEnumerator0" :`NewEnumerator0` "NewEnumerator1" :`NewEnumerator1` "NewEnumerator0" :`NewEnumerator2` "NewEnumerator0" :`NewEnumerator3` "NewEnumerator0" :`NewEnumerator4` "NewEnumerator0" :`NewEnumerator5` "NewEnumerator0" :`NewEnumerator6` "NewEnumerator0" :`NewEnumerator7` "NewEnumerator0" :`NewEnumerator8` "NewEnumerator0" :`NewEnumerator9` "NewEnumerator0" :`NewEnumerator10` "NewEnumerator0" :!type "/Game/Logic/Enumerators/E_SecretSkinSteps Enum") :!label _label_2)))

(event `Key|Up`
  (params (Key :type "Key Structure"))
  (:`Pressed`
    (goto _label_2)))

(event `Key|Gamepad_DPad_Down`
  (params (Key :type "Key Structure"))
  (:`Pressed`
    (`self.SetCurrentSkinStep` (select `/Game/Logic/Enumerators/E_SecretSkinSteps` (`self.SecretSkinStep`) :`NewEnumerator12` "NewEnumerator12" :`NewEnumerator0` "NewEnumerator12" :`NewEnumerator1` "NewEnumerator2" :`NewEnumerator2` "NewEnumerator3" :`NewEnumerator3` "NewEnumerator12" :`NewEnumerator4` "NewEnumerator12" :`NewEnumerator5` "NewEnumerator12" :`NewEnumerator6` "NewEnumerator12" :`NewEnumerator7` "NewEnumerator12" :`NewEnumerator8` "NewEnumerator12" :`NewEnumerator9` "NewEnumerator12" :`NewEnumerator10` "NewEnumerator12" :!type "/Game/Logic/Enumerators/E_SecretSkinSteps Enum") :!label _label_3)))

(event `Key|Down`
  (params (Key :type "Key Structure"))
  (:`Pressed`
    (goto _label_3)))

(event `Key|Gamepad_DPad_Left`
  (params (Key :type "Key Structure"))
  (:`Pressed`
    (`self.SetCurrentSkinStep` (select `/Game/Logic/Enumerators/E_SecretSkinSteps` (`self.SecretSkinStep`) :`NewEnumerator12` "NewEnumerator12" :`NewEnumerator0` "NewEnumerator12" :`NewEnumerator1` "NewEnumerator12" :`NewEnumerator2` "NewEnumerator12" :`NewEnumerator3` "NewEnumerator4" :`NewEnumerator4` "NewEnumerator12" :`NewEnumerator5` "NewEnumerator6" :`NewEnumerator6` "NewEnumerator12" :`NewEnumerator7` "NewEnumerator12" :`NewEnumerator8` "NewEnumerator12" :`NewEnumerator9` "NewEnumerator12" :`NewEnumerator10` "NewEnumerator12" :!type "/Game/Logic/Enumerators/E_SecretSkinSteps Enum") :!label _label_4)))

(event `Key|Left`
  (params (Key :type "Key Structure"))
  (:`Pressed`
    (goto _label_4)))

(event `Key|Gamepad_DPad_Right`
  (params (Key :type "Key Structure"))
  (:`Pressed`
    (`self.SetCurrentSkinStep` (select `/Game/Logic/Enumerators/E_SecretSkinSteps` (`self.SecretSkinStep`) :`NewEnumerator12` "NewEnumerator12" :`NewEnumerator0` "NewEnumerator12" :`NewEnumerator1` "NewEnumerator12" :`NewEnumerator2` "NewEnumerator12" :`NewEnumerator3` "NewEnumerator12" :`NewEnumerator4` "NewEnumerator5" :`NewEnumerator5` "NewEnumerator12" :`NewEnumerator6` "NewEnumerator7" :`NewEnumerator7` "NewEnumerator12" :`NewEnumerator8` "NewEnumerator12" :`NewEnumerator9` "NewEnumerator12" :`NewEnumerator10` "NewEnumerator12" :!type "/Game/Logic/Enumerators/E_SecretSkinSteps Enum") :!label _label_5)))

(event `Key|Right`
  (params (Key :type "Key Structure"))
  (:`Pressed`
    (goto _label_5)))

(event `Key|Gamepad_FaceButton_Right`
  (params (Key :type "Key Structure"))
  (:`Pressed`
    (`self.SetCurrentSkinStep` (select `/Game/Logic/Enumerators/E_SecretSkinSteps` (`self.SecretSkinStep`) :`NewEnumerator12` "NewEnumerator12" :`NewEnumerator0` "NewEnumerator12" :`NewEnumerator1` "NewEnumerator12" :`NewEnumerator2` "NewEnumerator12" :`NewEnumerator3` "NewEnumerator12" :`NewEnumerator4` "NewEnumerator12" :`NewEnumerator5` "NewEnumerator12" :`NewEnumerator6` "NewEnumerator12" :`NewEnumerator7` "NewEnumerator8" :`NewEnumerator8` "NewEnumerator12" :`NewEnumerator9` "NewEnumerator12" :`NewEnumerator10` "NewEnumerator12" :!type "/Game/Logic/Enumerators/E_SecretSkinSteps Enum") :!label _label_6)))

(event `Key|B`
  (params (Key :type "Key Structure"))
  (:`Pressed`
    (goto _label_6)))

(event `Key|Gamepad_FaceButton_Bottom`
  (params (Key :type "Key Structure"))
  (:`Pressed`
    (`self.SetCurrentSkinStep` (select `/Game/Logic/Enumerators/E_SecretSkinSteps` (`self.SecretSkinStep`) :`NewEnumerator12` "NewEnumerator12" :`NewEnumerator0` "NewEnumerator12" :`NewEnumerator1` "NewEnumerator12" :`NewEnumerator2` "NewEnumerator12" :`NewEnumerator3` "NewEnumerator12" :`NewEnumerator4` "NewEnumerator12" :`NewEnumerator5` "NewEnumerator12" :`NewEnumerator6` "NewEnumerator12" :`NewEnumerator7` "NewEnumerator12" :`NewEnumerator8` "NewEnumerator9" :`NewEnumerator9` "NewEnumerator12" :`NewEnumerator10` "NewEnumerator12" :!type "/Game/Logic/Enumerators/E_SecretSkinSteps Enum") :!label _label_7)
    (switch `/Game/Logic/Enumerators/E_SecretSkinSteps` (`self.SecretSkinStep`)
      (:`NewEnumerator9`
        (bind _returnvalue (`HIGameData.HIGetPlayerWerewolf`))
        (bind _asbp_vincent_volk (cast `/Game/Game_Files/Characters/Vincent_Volk/BP_Vincent_Volk` _returnvalue))
        (`/Game/Game_Files/Characters/Vincent_Volk/BP_Vincent_Volk.SwitchKatana` _asbp_vincent_volk)))))

(event `Key|A`
  (params (Key :type "Key Structure"))
  (:`Pressed`
    (goto _label_7)))

(fn `SetCurrentSkinStep`
  (params (SecretSkinStep :type "/Game/Logic/Enumerators/E_SecretSkinSteps Enum" :default "NewEnumerator12"))
  (set `self.SecretSkinStep` SecretSkinStep))

(fn `UserConstructionScript`)