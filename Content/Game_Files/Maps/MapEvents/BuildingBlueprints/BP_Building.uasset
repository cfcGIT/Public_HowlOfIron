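; BP_Building is a scalable building block for maps, with four BP_Wall child actors on its sides.
; The construction script clamps scale to at least 1, fits each wall to the block with per-wall offsets, and either swaps in a real mesh or shows the block with color-coded active/inactive labels.
; Wall data is pushed to the child walls, which also get reloaded, both at construction and on BeginPlay.
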(event `self.ReceiveBeginPlay`
  (`self.SetWallsData`)
  (`self.ReloadWalls`))

(fn `GetWall`
  (params (Target :type "ChildActorComponent Object Reference"))
  (returns (`AsBP Wall` :type "/Game/Game_Files/Maps/MapEvents/BuildingBlueprints/BP_Wall Object Reference"))
  (bind _asbp_wall (cast `/Game/Game_Files/Maps/MapEvents/BuildingBlueprints/BP_Wall` (`ChildActorComponent.ChildActor` Target)))
  (return _asbp_wall))

(fn `SetBackWall`
  (bind _back (`self.Back`))
  (bind (_returnvalue_x _returnvalue_y _returnvalue_z) (`KismetMathLibrary.BreakVector` (`SceneComponent.K2_GetComponentScale` (`self.staticMeshComponent`))))
  (`SceneComponent.SetWorldScale3D` _back (* (`SceneComponent.K2_GetComponentScale` _back) (`KismetMathLibrary.MakeVector` 1.0 _returnvalue_y _returnvalue_z)))
  (`SceneComponent.K2_SetWorldLocation` _back (+ (`SceneComponent.K2_GetComponentLocation` (`self.staticMeshComponent`)) (`KismetMathLibrary.MakeVector` (* (- 50.0 100.0) _returnvalue_x) (* 0.0 _returnvalue_y) (* 50.0 _returnvalue_z)) (* (`.LocationOffset_7_0C5C844B4BC7DA775B077DB511E4CA22` (break `/Game/Logic/Structures/S_Wall` (`self.BackWall`))) (-1.0 1.0 1.0))) false false))

(fn `SetFrontWall`
  (bind (_returnvalue_x _returnvalue_y _returnvalue_z) (`KismetMathLibrary.BreakVector` (`SceneComponent.K2_GetComponentScale` (`self.staticMeshComponent`))))
  (`SceneComponent.SetWorldScale3D` (`self.Front`) (* (`SceneComponent.K2_GetComponentScale` (`self.Front`)) (`KismetMathLibrary.MakeVector` 1.0 _returnvalue_y _returnvalue_z)))
  (`SceneComponent.K2_SetWorldLocation` (`self.Front`) (+ (`SceneComponent.K2_GetComponentLocation` (`self.staticMeshComponent`)) (`KismetMathLibrary.MakeVector` (* 50.0 _returnvalue_x) (* 0.0 _returnvalue_y) (* 50.0 _returnvalue_z)) (`.LocationOffset_7_0C5C844B4BC7DA775B077DB511E4CA22` (break `/Game/Logic/Structures/S_Wall` (`self.FrontWall`)))) false false))

(fn `SetLeftWall`
  (bind _left (`self.Left`))
  (bind (_returnvalue_x _returnvalue_y _returnvalue_z) (`KismetMathLibrary.BreakVector` (`SceneComponent.K2_GetComponentScale` (`self.staticMeshComponent`))))
  (`SceneComponent.SetWorldScale3D` _left (* (`SceneComponent.K2_GetComponentScale` _left) (`KismetMathLibrary.MakeVector` 1.0 _returnvalue_x _returnvalue_z)))
  (`SceneComponent.K2_SetWorldLocation` _left (+ (`SceneComponent.K2_GetComponentLocation` (`self.staticMeshComponent`)) (`KismetMathLibrary.MakeVector` (* 0.0 _returnvalue_x) (* (- 50.0 100.0) _returnvalue_y) (* 50.0 _returnvalue_z)) (`KismetMathLibrary.MakeVector` (.x (`.LocationOffset_7_0C5C844B4BC7DA775B077DB511E4CA22` (break `/Game/Logic/Structures/S_Wall` (`self.LeftWall`)))) (* (.y (`.LocationOffset_7_0C5C844B4BC7DA775B077DB511E4CA22` (break `/Game/Logic/Structures/S_Wall` (`self.LeftWall`)))) -1.0) (.z (`.LocationOffset_7_0C5C844B4BC7DA775B077DB511E4CA22` (break `/Game/Logic/Structures/S_Wall` (`self.LeftWall`)))))) false false))

(fn `SetRightWall`
  (bind _right (`self.Right`))
  (bind (_returnvalue_x _returnvalue_y _returnvalue_z) (`KismetMathLibrary.BreakVector` (`SceneComponent.K2_GetComponentScale` (`self.staticMeshComponent`))))
  (`SceneComponent.SetWorldScale3D` _right (* (`SceneComponent.K2_GetComponentScale` _right) (`KismetMathLibrary.MakeVector` 1.0 _returnvalue_x _returnvalue_z)))
  (`SceneComponent.K2_SetWorldLocation` _right (+ (`SceneComponent.K2_GetComponentLocation` (`self.staticMeshComponent`)) (`KismetMathLibrary.MakeVector` (* 0.0 _returnvalue_x) (* 50.0 _returnvalue_y) (* 50.0 _returnvalue_z)) (`.LocationOffset_7_0C5C844B4BC7DA775B077DB511E4CA22` (break `/Game/Logic/Structures/S_Wall` (`self.RightWall`)))) false false))

(fn `SetWallData`
  (params (TargetWall :type "ChildActorComponent Object Reference") (WallData :type "/Game/Logic/Structures/S_Wall Structure") (Text :type "TextRenderComponent Object Reference"))
  (bind _asbp_wall (cast `/Game/Game_Files/Maps/MapEvents/BuildingBlueprints/BP_Wall` (`ChildActorComponent.ChildActor` TargetWall)))
  (`/Game/Game_Files/Maps/MapEvents/BuildingBlueprints/BP_Wall.Set Wall Data` (`self.GetWall` TargetWall) WallData)
  (`/Game/Game_Files/Maps/MapEvents/BuildingBlueprints/BP_Wall.Set Wall Data` _asbp_wall WallData)
  (`TextRenderComponent.SetTextRenderColor` Text (select `bool` (`.IsActive_4_0C7A52904C4B5CC52D13618045C54D92` (break `/Game/Logic/Structures/S_Wall` WallData)) :`false` (make `Color` 0 0 255 255) :`true` (make `Color` 200 255 1 255))))

(fn `SetWallsData`
  (`self.SetWallData` (`self.Front`) (`self.FrontWall`) (`self.TextRender`))
  (`self.SetWallData` (`self.Back`) (`self.BackWall`) (`self.TextRender1`))
  (`self.SetWallData` (`self.Left`) (`self.LeftWall`) (`self.TextRender3`))
  (`self.SetWallData` (`self.Right`) (`self.RightWall`) (`self.TextRender2`)))

(fn `UserConstructionScript`
  (bind _blockmaterial (`self.BlockMaterial`))
  (bind _x (.x (`self.GetActorScale3D`)))
  (bind _y (.y (`self.GetActorScale3D`)))
  (bind _z (.z (`self.GetActorScale3D`)))
  (bind (_returnvalue_x _returnvalue_y) (`KismetMathLibrary.BreakVector` (`SceneComponent.K2_GetComponentScale` (`self.Left`))))
  (bind (_returnvalue_x_2 _returnvalue_y_2) (`KismetMathLibrary.BreakVector` (`SceneComponent.K2_GetComponentScale` (`self.Front`))))
  (bind (_returnvalue_x_3 _returnvalue_y_3) (`KismetMathLibrary.BreakVector` (`SceneComponent.K2_GetComponentScale` (`self.Front`))))
  (bind (_returnvalue_x_4 _returnvalue_y_4) (`KismetMathLibrary.BreakVector` (`SceneComponent.K2_GetComponentScale` (`self.Back`))))
  (bind (_returnvalue_x_5 _returnvalue_y_5) (`KismetMathLibrary.BreakVector` (`SceneComponent.K2_GetComponentScale` (`self.Right`))))
  (bind _returnvalue (* _returnvalue_y_5 (`self.TextScale`)))
  (bind _returnvalue_2 (* _returnvalue_y (`self.TextScale`)))
  (bind _returnvalue_3 (* _returnvalue_y_2 (`self.TextScale`)))
  (bind _returnvalue_4 (* _returnvalue_y_3 (`self.TextScale`)))
  (bind _returnvalue_5 (* _returnvalue_y_4 (`self.TextScale`)))
  (`self.ReloadWalls`)
  (`self.SetActorScale3D` (`KismetMathLibrary.MakeVector` (select `bool` (> _x 1.0) :`false` 1.0 :`true` _x) (select `bool` (> _y 1.0) :`false` 1.0 :`true` _y) (select `bool` (> _z 1.0) :`false` 1.0 :`true` _z)))
  (`PrimitiveComponent.SetMaterial` (`self.staticMeshComponent`) 0 (select `bool` (`KismetSystemLibrary.IsValid` _blockmaterial) :`false` "/Game/SuperGrid/StarterPack/Materials/Palette/Grids/M_SuperGrid_DefaultBlack.M_SuperGrid_DefaultBlack" :`true` _blockmaterial :!type "MaterialInterface Object Reference"))
  (`self.SetFrontWall`)
  (`self.SetBackWall`)
  (`self.SetLeftWall`)
  (`self.SetRightWall`)
  (`self.SetWallsData`)
  (if (`self.ShowRealMesh`)
    (`/Engine/EditorBlueprintResources/StandardMacros.IsValid` (`self.Mesh`)
      (:`Is Valid`
        (`StaticMeshComponent.SetStaticMesh` (`self.BuildingMesh`) (`self.Mesh`))
        (`SceneComponent.SetVisibility` (`self.BuildingMesh`) true false)
        (`SceneComponent.SetVisibility` (`self.staticMeshComponent`) false false)
        (`SceneComponent.SetVisibility` (`self.TextRender3`) false false)
        (`SceneComponent.SetVisibility` (`self.TextRender2`) false false)
        (`SceneComponent.SetVisibility` (`self.TextRender1`) false false)
        (`SceneComponent.SetVisibility` (`self.TextRender`) false false)))
    (else
      (`SceneComponent.SetVisibility` (`self.BuildingMesh`) false false)
      (`SceneComponent.SetVisibility` (`self.staticMeshComponent`) true false)
      (`SceneComponent.SetWorldScale3D` (`self.TextRender`) (`KismetMathLibrary.MakeVector` _returnvalue_3 _returnvalue_3 _returnvalue_3))
      (`SceneComponent.SetWorldScale3D` (`self.TextRender`) (`KismetMathLibrary.MakeVector` _returnvalue_4 _returnvalue_4 _returnvalue_4))
      (`SceneComponent.SetWorldScale3D` (`self.TextRender1`) (`KismetMathLibrary.MakeVector` _returnvalue_5 _returnvalue_5 _returnvalue_5))
      (`SceneComponent.SetWorldScale3D` (`self.TextRender2`) (`KismetMathLibrary.MakeVector` _returnvalue _returnvalue _returnvalue))
      (`SceneComponent.SetWorldScale3D` (`self.TextRender3`) (`KismetMathLibrary.MakeVector` _returnvalue_2 _returnvalue_2 _returnvalue_2))
      (`SceneComponent.SetVisibility` (`self.TextRender3`) true false)
      (`SceneComponent.SetVisibility` (`self.TextRender2`) true false)
      (`SceneComponent.SetVisibility` (`self.TextRender1`) true false)
      (`SceneComponent.SetVisibility` (`self.TextRender`) true false))))