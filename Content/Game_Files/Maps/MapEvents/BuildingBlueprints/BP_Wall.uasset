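; BP_Wall is a map building wall that can be toggled climbable or non-climbable.
; SetWallData takes the active flag from the supplied wall data, stores it as IsClimbable and switches the box's response on a custom trace channel between Block and Ignore.
; The construction script and SetWallData both color the Area component blue or red with debug materials to show that state, and fix its scale.
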(fn `Set Wall Data`
  (params (WallData :type "/Game/Logic/Structures/S_Wall Structure"))
  (bind _isactive (break `/Game/Logic/Structures/S_Wall` WallData))
  (`PrimitiveComponent.SetCollisionResponseToChannel` (`self.boxComponent`) "ECC_GameTraceChannel3" (select `bool` _isactive :`false` "ECR_Ignore" :`true` "ECR_Block" :!type "ECollisionResponse Enum"))
  (set `self.isClimbable` _isactive)
  (`PrimitiveComponent.SetMaterial` (`self.Area`) 0 (select `bool` (`self.isClimbable`) :`false` "/Game/Logic/LevelDesign_Utilities/Materials/Debug/M_DebugMaterial_Red.M_DebugMaterial_Red" :`true` "/Game/Logic/LevelDesign_Utilities/Materials/Debug/M_DebugMaterial_Blue.M_DebugMaterial_Blue" :!type "MaterialInterface Object Reference"))
  (`SceneComponent.SetRelativeScale3D` (`self.Area`) (0.641 0.641 0.641)))

(fn `UserConstructionScript`
  (`SceneComponent.SetRelativeScale3D` (`self.Area`) (0.641 0.641 0.641))
  (`PrimitiveComponent.SetMaterial` (`self.Area`) 0 (select `bool` (`self.isClimbable`) :`false` "/Game/Logic/LevelDesign_Utilities/Materials/Debug/M_DebugMaterial_Red.M_DebugMaterial_Red" :`true` "/Game/Logic/LevelDesign_Utilities/Materials/Debug/M_DebugMaterial_Blue.M_DebugMaterial_Blue" :!type "MaterialInterface Object Reference"))
  (`SceneComponent.SetRelativeScale3D` (`self.Area`) (0.641 0.641 0.641)))