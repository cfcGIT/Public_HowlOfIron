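; BP_sOUNDpOINT is a map event that plays a dialogue line from its first enemy when its condition check passes.
; On success it builds a delegate stop condition wrapping an OR of an in-combat condition and an event condition attached to that enemy's death.
; That stop condition is passed with SoundRow to HIPlayDialogue, so combat or the speaker's death can cut the dialogue short.
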(event `self.HIOnConditionChecked`
  (params (conditionResult :type Boolean))
  (if conditionResult
    (bind _returnvalue (`|GenericCreateObject` "/Script/HowlOfIron.HIDelegateCondition" self))
    (bind _output_get (set `self.StopCondition` _returnvalue))
    (bind _returnvalue_2 (`|GenericCreateObject` "/Script/HowlOfIron.HIInCombatCondition" _output_get))
    (bind _returnvalue_3 (`|GenericCreateObject` "/Script/HowlOfIron.HIEventCondition" (`self.StopCondition`)))
    (`HIEventCondition.AttachToEnemyDeath` _returnvalue_3 (`self.HIGetFirstEnemy`))
    (bind _returnvalue_4 (`|GenericCreateObject` "/Script/HowlOfIron.HIORCondition" (`self.StopCondition`)))
    (`HIORCondition.HIAddCondition` _returnvalue_4 _returnvalue_2)
    (`HIORCondition.HIAddCondition` _returnvalue_4 _returnvalue_3)
    (`HIDelegateCondition.HISetCondition` _output_get _returnvalue_4)
    (`HIAudio.HIPlayDialogue` (`self.HIGetFirstEnemy`) (`self.Sound Row`) (`self.StopCondition`))))

(fn `UserConstructionScript`)