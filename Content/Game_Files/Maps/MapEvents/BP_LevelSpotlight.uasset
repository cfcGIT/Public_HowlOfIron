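; BP_LevelSpotlight is a level spotlight actor with optional flickering and back-and-forth rotation, each enabled by its own flag.
; Flicker cuts intensity to zero for a random interval, restores it, then re-arms a randomly timed one-shot timer.
; For rotation, a looping timer plays or reverses a timeline that lerps the actor between two rotations, flipping direction after a stop delay at each end.
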(event `ResetTimer`
  (bind (_flickertimerange_x _flickertimerange_y) (`KismetMathLibrary.BreakVector2D` (`self.flickerTimeRange`)))
  ;[1 1 1] Flickering
  (`KismetSystemLibrary.K2_SetTimerDelegate` (delegate `LightFlicker`) (`KismetMathLibrary.RandomFloatInRange` _flickertimerange_x _flickertimerange_y) :!label _label))

(event `self.ReceiveBeginPlay`
  (`|ExecutionSequence`
    (:`then_0`
      ;[1 1 1] Flickering
      (if (`self.isFlickering`)
        (goto _label)))
    (:`then_1`
      ;[1 1 1] Rotation
      (if (`self.isRotating`)
        (`KismetSystemLibrary.K2_SetTimerDelegate` (delegate `RotateLight`) 0.5 true)))))

(event `LightFlicker`
  ;[1 1 1] Flickering
  (`self.SimpleFlick`))

(event `SimpleFlick`
  (bind (_offtimeflicker_x _offtimeflicker_y) (`KismetMathLibrary.BreakVector2D` (`self.offTimeFlicker`)))
  (bind _lightcomponent (`self.LightComponent`))
  ;[1 1 1] Flickering
  ;;[0.04314 0.04314 0.04314] Simple Flicker ON/OFF
  (set `self.IntensityBackup` (`LightComponentBase.Intensity` _lightcomponent))
  (`LightComponent.SetIntensity` _lightcomponent 0.0)
  (`KismetSystemLibrary.Delay` (`KismetMathLibrary.RandomFloatInRange` _offtimeflicker_x _offtimeflicker_y))
  (`LightComponent.SetIntensity` _lightcomponent (`self.IntensityBackup`))
  (`self.ResetTimer`))

(event `RotateLight`
  ;[1 1 1] Rotation
  ;;[0.04688 0.04688 0.04688] Rotate Light
  (if (`self.rightRotation`)
    (bind (_direction _z) (`Timeline|Rotation_Z` :!label _label_2)
      (:`Update`
        (`self.K2_SetActorRotation` self (`KismetMathLibrary.RLerp` (`self.rotationRange_A`) (`self.rotationRange_B`) _z) false))
      (:`Finished`
        (`KismetSystemLibrary.Delay` (`self.StopTime`))
        (set `self.rightRotation` (not (`self.rightRotation`)))))
    (else
      (goto _label_2 :!via `Reverse`))))

(fn `UserConstructionScript`)