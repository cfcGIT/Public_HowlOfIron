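; BP_CustomTrigger is a level design utility trigger with a color-coded debug collider.
; Its construction script runs the parent's, then resets DebugCollider's relative location to the origin.
; It creates a dynamic instance of each collider material and sets the "Color" parameter to CustomEnabledColor.
; The event graph holds only disabled stubs, so the Blueprint adds no runtime logic of its own.
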(fn `UserConstructionScript`
  (bind _debugcollider (`self.debugCollider`))
  (bind _returnvalue (`MeshComponent.GetMaterials` _debugcollider))
  (`parent.UserConstructionScript`)
  (`SceneComponent.K2_SetRelativeLocation` (`self.debugCollider`) (0.0 0.0 0.0) false false)
  (for (_array_element _array_index) _returnvalue
    (if (`KismetArrayLibrary.Array_IsValidIndex` _returnvalue _array_index)
      (bind _returnvalue_2 (`PrimitiveComponent.CreateDynamicMaterialInstance` _debugcollider _array_index _array_element "None"))
      (`MaterialInstanceDynamic.SetVectorParameterValue` _returnvalue_2 "Color" (`self.CustomEnabledColor`)))))