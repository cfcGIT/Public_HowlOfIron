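; BP_MeshReplacer is a level design utility that swaps one static mesh for another across the world's StaticMeshActors.
; Its ReplaceStaticMeshes event checks that both meshes are valid, then scans every StaticMeshActor and assigns NewMesh wherever PreviousMesh is used.
; With UseCustomRotation enabled, it also adds CustomRotation to each replaced actor's current rotation, component by component.
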(event `self.ReplaceStaticMeshes`
  (bind (_customrotation_roll _customrotation_pitch _customrotation_yaw) (`KismetMathLibrary.BreakRotator` (`self.customRotation`)))
  ;[0 0 0] Replace Static Meshes
  (if (and (`KismetSystemLibrary.IsValid` (`self.previousMesh`)) (`KismetSystemLibrary.IsValid` (`self.newMesh`)))
    (bind _outactors (`GameplayStatics.GetAllActorsOfClass` "/Script/Engine.StaticMeshActor"))
    (for _array_element _outactors
      (bind _staticmeshcomponent (`StaticMeshActor.StaticMeshComponent` _array_element))
      (if (== (`StaticMeshComponent.StaticMesh` _staticmeshcomponent) (`self.previousMesh`))
        (`StaticMeshComponent.SetStaticMesh` _staticmeshcomponent (`self.newMesh`))
        (if (`self.bUseCustomRotation`)
          (`self.K2_SetActorRotation` _array_element (`KismetMathLibrary.MakeRotator` (+ (.roll (`self.K2_GetActorRotation` _array_element)) _customrotation_roll) (+ (.pitch (`self.K2_GetActorRotation` _array_element)) _customrotation_pitch) (+ (.yaw (`self.K2_GetActorRotation` _array_element)) _customrotation_yaw)) false))))))

(fn `UserConstructionScript`)