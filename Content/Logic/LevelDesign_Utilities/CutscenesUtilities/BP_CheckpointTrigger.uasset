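; BP_CheckpointTrigger is a level-design trigger that records a checkpoint when the player character Vincent Volk overlaps its box.
; It checks its display name against the reached checkpoints in the game instance to avoid triggering again.
; For a new checkpoint, a DoOnce registers the name, sets checkpoint data from the referenced player start's tag and shows the save-game icon on the player's widget.
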(event `self.Box.OnComponentBeginOverlap`
  (params (OverlappedComponent :type "PrimitiveComponent Object Reference") (OtherActor :type "Actor Object Reference") (OtherComp :type "PrimitiveComponent Object Reference") (OtherBodyIndex :type Integer) (bFromSweep :type Boolean) (SweepResult :type "HitResult Structure (by ref)"))
  (bind _asbp_vincent_volk (cast `/Game/Game_Files/Characters/Vincent_Volk/BP_Vincent_Volk` OtherActor))
  (set `self.Werewolf` _asbp_vincent_volk)
  ;[0.01 0.01 0.01] Event Save Game on Overlap
  (bind _asbp_higame_instance (cast `/Game/Logic/Scripts/Game/BP_HIGameInstance` (`GameplayStatics.GetGameInstance`)))
  (bind _checkpoints (`/Game/Logic/Scripts/Game/BP_HIGameInstance.GetReachedCheckpoints` _asbp_higame_instance))
  (if (> (`KismetArrayLibrary.Array_Length` _checkpoints) 0)
    (for _array_element _checkpoints
      (if (`KismetStringLibrary.EqualEqual_StrStr` _array_element (`KismetSystemLibrary.GetDisplayName` self))
        (set `self.Triggered` true)
        (break))))
  (if (not (`self.Triggered`))
    (`/Engine/EditorBlueprintResources/StandardMacros.DoOnce` false
      (:`Completed`
        (bind _asbp_higame_instance_2 (cast `/Game/Logic/Scripts/Game/BP_HIGameInstance` (`GameplayStatics.GetGameInstance`))
          (:`then`
            (`/Game/Logic/Scripts/Game/BP_HIGameInstance.AddReachedCheckpoint` _asbp_higame_instance_2 (`KismetSystemLibrary.GetDisplayName` self)))
          (:`CastFailed`
            _))
        (`/Game/Logic/LevelDesign_Utilities/FL_LevelDesignFunctions.SetCheckpointData` (`PlayerStart.PlayerStartTag` (`self.CheckpointReference`)))
        (message `/Game/Logic/Interfaces/BI_ManagementHUD.ShowSaveGameIcon` (`HIWerewolf.widgetref` (`self.Werewolf`)))))))

(fn `UserConstructionScript`)