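; Trigger volume that plays a Level Sequence cutscene when Vincent Volk overlaps it, skipping triggers already recorded by display name in the game instance.
; Playback pauses enemies, applies a cinematic GameplayEffect, shows the cutscene HUD, lowers or overrides music volume, and runs optional per-level hiding, moving and cleanup tweaks.
; A timer matching sequence length drives EndCutscene, which restores input, enemies, rain and audio, and swaps the soundtrack.
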(event `self.ReceiveBeginPlay`)

(event `Event PlayCutscene`
  (params (Werewolf :type "/Game/Game_Files/Characters/Vincent_Volk/BP_Vincent_Volk Object Reference"))
  (set `self.Werewolf` Werewolf)
  ;[0.3021 0.0755 0.0785] Play Sequence
  (bind _outactors (`GameplayStatics.GetAllActorsOfClass` "/Game/Assets/Rain_FX/RainFX_Tools/BP_Rain_M.BP_Rain_M_C" :!label _label))
  (`/Game/Assets/Rain_FX/RainFX_Tools/BP_Rain_M.CutsceneRain` (`|GetArrayItem` _outactors))
  (bind _asbp_vincent_volk_controller (cast `/Game/Game_Files/Characters/Vincent_Volk/BP_VincentVolkController` (`GameplayStatics.GetPlayerController` 0)))
  (set `/Game/Game_Files/Characters/Vincent_Volk/BP_VincentVolkController.CanSkip` (`self.CanSkip`) _asbp_vincent_volk_controller)
  (bind _asbp_higame_instance (cast `/Game/Logic/Scripts/Game/BP_HIGameInstance` (`GameplayStatics.GetGameInstance`)))
  (bind _cutscenetriggers (`/Game/Logic/Scripts/Game/BP_HIGameInstance.GetCutsceneTriggers` _asbp_higame_instance))
  (if (> (`KismetArrayLibrary.Array_Length` _cutscenetriggers) 0)
    (for _array_element _cutscenetriggers
      (if (`KismetStringLibrary.EqualEqual_StrStr` _array_element (`KismetSystemLibrary.GetDisplayName` self))
        (set `self.CutsceneTriggered` true)
        (break))))
  (if (not (`self.CutsceneTriggered`))
    (`/Engine/EditorBlueprintResources/StandardMacros.DoOnce` false
      (:`Completed`
        (bind _asbp_higame_instance_2 (cast `/Game/Logic/Scripts/Game/BP_HIGameInstance` (`GameplayStatics.GetGameInstance`))
          (:`then`
            (`/Game/Logic/Scripts/Game/BP_HIGameInstance.AddCutsceneTrigger` _asbp_higame_instance_2 (`KismetSystemLibrary.GetDisplayName` self)))
          (:`CastFailed`
            _))
        (`HIGameData.HIPauseEnemies`)
        (`|ExecutionSequence`
          (:`then_0`
            (bind _returnvalue (`AbilitySystemComponent.BP_ApplyGameplayEffectToSelf` :`self` (`HIAbilityCharacter.abilitySystem` (`self.Werewolf`)) :`GameplayEffectClass` "/Game/Game_Files/Characters/Vincent_Volk/Abilities/GameplayEffects/DisableInputs/GE_CinematicMode.GE_CinematicMode_C"))
            (set `self.DisbaleInput` _returnvalue)
            (bind (_outactor _returnvalue_2) (`LevelSequencePlayer.CreateLevelSequencePlayer` (`self.LevelSequenceToPlay`)))
            (set `self.SequencePlayer` _returnvalue_2)
            (`MovieSceneSequencePlayer.Play` _returnvalue_2)
            (`self.Event ShowCutsceneHUD`)
            (bind _returnvalue_3 (`TimeManagementBlueprintLibrary.Conv_QualifiedFrameTimeToSeconds` (`MovieSceneSequencePlayer.GetEndTime` _returnvalue_2)))
            (set `self.Time` _returnvalue_3)
            (bind _returnvalue_4 (`KismetSystemLibrary.K2_SetTimerDelegate` (`|CreateDelegate` :!event `Event EndCutscene`) _returnvalue_3))
            (set `self.CutsceneTimer` _returnvalue_4))
          (:`then_1`
            (if (`self.SetCenterCinematic`)
              (`KismetSystemLibrary.Delay` 1.0)
              (`self.K2_SetActorLocation` (`GameplayStatics.GetPlayerCharacter` 0) (`PrimitiveComponent.GetCenterOfMass` (`self.Box`) "None") false false)))
          (:`then_2`
            (if (`self.BoolLightsOnOff`)
              (for _array_element_2 (`self.LightsOnOff`)
                (`self.SetActorHiddenInGame` _array_element_2 false))))
          (:`then_3`
            (if (`self.DeleteMesh`)
              (bind _outactors_2 (`GameplayStatics.GetAllActorsWithTag` (`self.MuttonToDelete`)))
              (`self.K2_DestroyActor` (`|GetArrayItem` _outactors_2))))
          (:`then_4`
            (`GameplayStatics.SetSoundMixClassOverride` "/Game/Game_Files/SFX/Mixer/SM_Mixer.SM_Mixer" "/Game/Game_Files/SFX/Mixer/SC_Music.SC_Music" (`self.MusicVolume`)))
          (:`then_5`
            (if (`self.Hide Wolf`)
              (`KismetSystemLibrary.Delay` (`self.Hidden Time`))
              (`self.SetActorHiddenInGame` (`self.Werewolf`) true)))
          (:`then_6`
            (if (`self.MoveWolf`)
              (`self.K2_SetActorLocation` (`self.Werewolf`) (4896.0 2498.0 38.0) false false)))
          (:`then_7`
            (if (`self.HideBoss`)
              (`self.SetActorHiddenInGame` (`self.Werewolf`) true)
              (`KismetSystemLibrary.Delay` (`self.Hidden Time`))
              (`self.SetActorHiddenInGame` (`self.Werewolf`) false))))))))

(event `self.Box.OnComponentBeginOverlap`
  (params (OverlappedComponent :type "PrimitiveComponent Object Reference") (OtherActor :type "Actor Object Reference") (OtherComp :type "PrimitiveComponent Object Reference") (OtherBodyIndex :type Integer) (bFromSweep :type Boolean) (SweepResult :type "HitResult Structure (by ref)"))
  ;[0.3021 0.0755 0.0785] Play Sequence
  (bind _asbp_vincent_volk (cast `/Game/Game_Files/Characters/Vincent_Volk/BP_Vincent_Volk` OtherActor))
  (set `self.Werewolf` _asbp_vincent_volk)
  (goto _label))

(event `Event EndCutscene`
  ;[0.3021 0.0755 0.0785] Play Sequence
  (`KismetSystemLibrary.K2_ClearAndInvalidateTimerHandle` (`self.CutsceneTimer`))
  (`|ExecutionSequence`
    (:`then_0`
      (bind _asbp_higame_instance (cast `/Game/Logic/Scripts/Game/BP_HIGameInstance` (`GameplayStatics.GetGameInstance`)))
      (`GameplayStatics.SetSoundMixClassOverride` "/Game/Game_Files/SFX/Mixer/SM_Mixer.SM_Mixer" "/Game/Game_Files/SFX/Mixer/SC_Music.SC_Music" (`HIGameInstance.ambientValue` _asbp_higame_instance))
      (`/Game/Logic/BP_HIAmbientSound.ChangeCurrentSoundtrack` (`self.GetAmbientSound`) (`self.New Hunt Music`) (`self.New Combat Music`))
      (bind _outactors (`GameplayStatics.GetAllActorsOfClass` "/Game/Assets/Rain_FX/RainFX_Tools/BP_Rain_M.BP_Rain_M_C"))
      (bind _output (`|GetArrayItem` _outactors))
      (`/Game/Assets/Rain_FX/RainFX_Tools/BP_Rain_M.NormalRain` _output)
      (`/Game/Assets/Rain_FX/RainFX_Tools/BP_Rain_M.TurnAlarmOn` _output (`self.TurnAlarmSoundOn`))
      (`AbilitySystemComponent.RemoveActiveGameplayEffect` (`HIAbilityCharacter.abilitySystem` (`self.Werewolf`)) (`self.DisbaleInput`) -1)
      (`self.Event HideCutsceneHUD`)
      (`HIGameData.HIResumeEnemies`)
      (`self.OnFinishCutscene`)
      (if (`MovieSceneSequencePlayer.IsPlaying` (`self.SequencePlayer`))
        (`MovieSceneSequencePlayer.GoToEndAndStop` (`self.SequencePlayer`))))
    (:`then_1`
      (if (`self.HideBoss`)
        (bind _asbp_vincent_volk_boss (cast `/Game/Game_Files/Characters/Vincent_Volk/BP_Vincent_Volk_Boss` (`self.Werewolf`)))
        (`self.SetActorHiddenInGame` _asbp_vincent_volk_boss false)))
    (:`then_2`
      (if (`self.Hide Wolf`)
        (`self.SetActorHiddenInGame` (`self.Werewolf`) false)))
    (:`then_3`
      (if (`self.ShowBossHud`)
        (bind _returnvalue (`GameplayStatics.GetActorOfClass` "/Game/Game_Files/Characters/Enemies/Hunter/BP_Hunter.BP_Hunter_C"))
        (`/Game/Game_Files/Characters/Enemies/Hunter/BP_Hunter.ShowHUD` _returnvalue)))))

(event `Event ShowCutsceneHUD`
  ;[0.0625 0.0625 0.0625] Cutscene BlackHUD
  (bind _ashiwerewolf (cast `HIWerewolf` (`GameplayStatics.GetPlayerCharacter` 0)))
  (message `/Game/Logic/Interfaces/BI_ManagementHUD.OpenCutscene` (`HIWerewolf.widgetref` _ashiwerewolf) self))

(event `Event HideCutsceneHUD`
  ;[0.0625 0.0625 0.0625] Cutscene BlackHUD
  (bind _ashiwerewolf (cast `HIWerewolf` (`GameplayStatics.GetPlayerCharacter` 0)))
  (message `/Game/Logic/Interfaces/BI_ManagementHUD.CloseCutscene` (`HIWerewolf.widgetref` _ashiwerewolf)))

(event `Event LoadEndDemo`
  (params (Level :type String)))

(fn `GetAmbientSound`
  (returns (`Ambient Sound` :type "/Game/Logic/BP_HIAmbientSound Object Reference"))
  (bind _returnvalue (`HIGameData.HIGetSpeaker2D`))
  (bind _asbp_hiambient_sound (cast `/Game/Logic/BP_HIAmbientSound` _returnvalue))
  (return _asbp_hiambient_sound))

(fn `UserConstructionScript`)