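; Game mode that spawns the player at the PlayerStart matching the saved checkpoint.
; The ChoosePlayerStart override clears static references, then compares each PlayerStart's tag to the checkpoint data.
; Without a match, it falls back to the start tagged as the first checkpoint, or else to the first one found.
; BeginPlay copies reached checkpoints and cutscene triggers from BP_HIGameInstance into local variables.
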(event `self.ReceiveBeginPlay`
  (bind _asbp_higame_instance (cast `/Game/Logic/Scripts/Game/BP_HIGameInstance` (`GameplayStatics.GetGameInstance`)))
  (bind _checkpoints (`/Game/Logic/Scripts/Game/BP_HIGameInstance.GetReachedCheckpoints` _asbp_higame_instance))
  (set `self.AuxCheckpoints` _checkpoints)
  (bind _cutscenetriggers (`/Game/Logic/Scripts/Game/BP_HIGameInstance.GetCutsceneTriggers` _asbp_higame_instance))
  (set `self.AuxCutsceneTriggers` _cutscenetriggers))

(fn `ChoosePlayerStart`
  (params (Player :type "Controller Object Reference"))
  (returns (ReturnValue :type "Actor Object Reference"))
  (locals (FirstCheckpoint :type "PlayerStart Object Reference") (TargetCheckpoint :type "PlayerStart Object Reference") (CurrentArrayCheckpoint :type "PlayerStart Object Reference"))
  ;[0.01 0.01 0.01] Choose Player Start
  (`HIGameData.HIClearStaticReferences`)
  (bind _outactors (`GameplayStatics.GetAllActorsOfClass` "/Script/Engine.PlayerStart"))
  (for _array_element _outactors
    (set `local.CurrentArrayCheckpoint` _array_element)
    (if (== (`PlayerStart.PlayerStartTag` _array_element) (`/Game/Logic/LevelDesign_Utilities/FL_LevelDesignFunctions.GetCheckpointData`))
      (set `local.TargetCheckpoint` (`local.CurrentArrayCheckpoint`))
      (break)
      (elif (== (`PlayerStart.PlayerStartTag` (`local.CurrentArrayCheckpoint`)) "Checkpoint1")
        (set `local.FirstCheckpoint` (`local.CurrentArrayCheckpoint`)))))
  (if (!= (`local.TargetCheckpoint`) null)
    (return (`local.TargetCheckpoint`))
    (else
      (bind _outactors_2 (`GameplayStatics.GetAllActorsOfClass` "/Script/Engine.PlayerStart"))
      (return (select `bool` (`KismetSystemLibrary.IsValid` (`local.FirstCheckpoint`)) :`false` (`|GetArrayItem` _outactors_2) :`true` (`local.FirstCheckpoint`) :!type "Actor Object Reference")))))

(fn `UserConstructionScript`)