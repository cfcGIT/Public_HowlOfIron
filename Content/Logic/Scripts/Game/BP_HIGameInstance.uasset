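; Game instance that holds checkpoint, level and cutscene progress, plus controller type, subtitle and katana mode settings, and shows HI tooltips.
; New triggers and checkpoints collect in the game mode's Aux lists until InitCheckpoint copies them in and saves to an SG_SaveGame slot.
; Changing level resets progress and saves.
; Loading restores only checkpoint tag and level, as the restore of both lists is unconnected.
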(event `self.HIShowTooltip`
  (params (rowName :type Name))
  ;[0.01 0.01 0.01] Event Show Tooltip
  (`self.HIActivateTooltip` rowName)
  (bind _returnvalue (`self.HIGetTooltipWidget`))
  (`Widget.SetVisibility` _returnvalue "Visible"))

(fn `AddCutsceneTrigger`
  (params (NewCutsceneTriggerName :type "String (by ref)"))
  (bind _asbp_hi_game_mode (cast `/Game/Logic/Scripts/Game/BP_HI_GameMode` (`GameplayStatics.GetGameMode`)))
  (`KismetArrayLibrary.Array_Add` (`/Game/Logic/Scripts/Game/BP_HI_GameMode.AuxCutsceneTriggers` _asbp_hi_game_mode) NewCutsceneTriggerName))

(fn `AddReachedCheckpoint`
  (params (NewCheckpoint :type "String (by ref)"))
  (bind _asbp_hi_game_mode (cast `/Game/Logic/Scripts/Game/BP_HI_GameMode` (`GameplayStatics.GetGameMode`)))
  (`KismetArrayLibrary.Array_Add` (`/Game/Logic/Scripts/Game/BP_HI_GameMode.AuxCheckpoints` _asbp_hi_game_mode) NewCheckpoint))

(fn `ClearSavedData`
  (set `self.CheckpointTag` "None")
  (set `self.CurrentLevel` "Lvl_Steelheart")
  (`KismetArrayLibrary.Array_Clear` (`self.CutsceneTriggers`))
  (`KismetArrayLibrary.Array_Clear` (`self.Checkpoints`)))

(fn `DeleteSaveData`
  (`GameplayStatics.DeleteGameInSlot` (`self.SaveGameSlotName`)))

(fn `GetCheckpointData`
  (returns (CheckpointTag :type Name))
  (return (`self.CheckpointTag`)))

(fn `GetControllerType`
  (returns (Controller :type "/Game/Logic/Enumerators/E_Controller Enum"))
  (return (`self.Controller`)))

(fn `GetCutsceneTriggers`
  (returns (CutsceneTriggers :type "Array of String"))
  (return (`self.CutsceneTriggers`)))

(fn `GetKatanaMode`
  (returns (KatanaMode :type Boolean))
  (return (`self.KatanaMode`)))

(fn `GetReachedCheckpoints`
  (returns (Checkpoints :type "Array of String"))
  (return (`self.Checkpoints`)))

(fn `GetShowSubtitles`
  (returns (ShowSubtitles :type Boolean))
  (return (`self.ShowSubtitles`)))

(fn `InitCheckpoint`
  (params (CheckpointTag :type Name))
  ;[0.01 0.01 0.01] Init Checkpoint
  (set `self.CheckpointTag` CheckpointTag)
  (bind _asbp_hi_game_mode (cast `/Game/Logic/Scripts/Game/BP_HI_GameMode` (`GameplayStatics.GetGameMode`)))
  (set `self.CutsceneTriggers` (`/Game/Logic/Scripts/Game/BP_HI_GameMode.AuxCutsceneTriggers` _asbp_hi_game_mode))
  (set `self.Checkpoints` (`/Game/Logic/Scripts/Game/BP_HI_GameMode.AuxCheckpoints` _asbp_hi_game_mode))
  (`self.SaveGameData`))

(fn `LoadSaveData`
  (bind _savegame (`self.SaveGame`))
  (`|ExecutionSequence`
    (:`then_0`
      (bind _returnvalue (`GameplayStatics.DoesSaveGameExist` (`self.SaveGameSlotName`)))
      (if _returnvalue
        (bind _returnvalue_2 (`GameplayStatics.LoadGameFromSlot` (`self.SaveGameSlotName`)))
        (bind _assg_save_game (cast `/Game/Logic/Scripts/Game/SG_SaveGame` _returnvalue_2))
        (set `self.SaveGame` _assg_save_game)
        (else
          (bind _returnvalue_3 (`GameplayStatics.CreateSaveGameObject` "/Game/Logic/Scripts/Game/SG_SaveGame.SG_SaveGame_C"))
          (set `self.SaveGame` _returnvalue_3))))
    (:`then_1`
      (set `self.CheckpointTag` (`/Game/Logic/Scripts/Game/SG_SaveGame.CheckpointTag` _savegame))
      (set `self.CurrentLevel` (`/Game/Logic/Scripts/Game/SG_SaveGame.CurrentLevel` _savegame)))))

(fn `SaveGameData`
  (bind _savegame (`self.SaveGame`)
    (:`then`
      (`/Game/Logic/Scripts/Game/SG_SaveGame.SetParams` _savegame (`self.CheckpointTag`) (`self.CurrentLevel`) (`self.CutsceneTriggers`) (`self.Checkpoints`))
      (`GameplayStatics.SaveGameToSlot` (`self.SaveGame`) (`self.SaveGameSlotName`)))
    (:`else`)))

(fn `SetControllerType`
  (params (Controller :type "/Game/Logic/Enumerators/E_Controller Enum" :default "NewEnumerator0"))
  (set `self.Controller` Controller))

(fn `SetCurrentLevel`
  (params (CurrentLevel :type Name))
  (set `self.CurrentLevel` CurrentLevel)
  (set `self.CheckpointTag` "None")
  (`KismetArrayLibrary.Array_Clear` (`self.CutsceneTriggers`))
  (`KismetArrayLibrary.Array_Clear` (`self.Checkpoints`))
  (`self.SaveGameData`))

(fn `SetKatanaMode`
  (params (KatanaMode :type Boolean))
  (set `self.KatanaMode` KatanaMode))

(fn `SetShowSubtitles`
  (params (ShowSubtitles :type Boolean :default true))
  (set `self.ShowSubtitles` ShowSubtitles))