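; Ambient music controller that switches between hunt and combat music and plays menu music in the main menu.
; Tracks load by row name from an audio data table and crossfade on state changes.
; Each intro binds OnAudioFinished to start its loop, then unbinds.
; ChangeCurrentSoundtrack swaps intro names and picks the Bridge or Hunter loop/outro set from the combat intro name; pause playback only prints a debug string.
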(event `self.ReceiveBeginPlay`
  (if (`KismetSystemLibrary.IsValid` (`self.actualComponent`))
    (`AudioComponent.Stop` (`self.actualComponent`)))
  (if (`self.isMainMenu`)
    (`self.HIPlayMusic` "HuntMusic" (`self.pauseMusic`) 2.0)
    (else
      (`self.HIPlayMusic` "HuntMusic" (`self.huntMusic`) 2.0))))

(event `self.HIStartMusics`
  (bind _actualcomponent (`self.actualComponent`))
  (`self.HISetHuntMusic` (make `DataTableRowHandle` "/Game/Logic/DataTables/CDT_Audio.CDT_Audio" (`self.Hunt Music Intro`)))
  (`self.HISetCombatMusic` (make `DataTableRowHandle` "/Game/Logic/DataTables/CDT_Audio.CDT_Audio" (`self.Combat Music Intro`)))
  (`self.HISetPausetMusic` (make `DataTableRowHandle` "/Game/Logic/DataTables/CDT_Audio.CDT_Audio" (`self.Menu Music`)))
  (if (`KismetSystemLibrary.IsValid` _actualcomponent)
    (`AudioComponent.Stop` _actualcomponent)))

(event `self.HIPlayCombat`
  (bind _actualcomponent (`self.actualComponent`))
  (bind _actualcomponent_2 (`self.actualComponent`))
  (`/Engine/EditorBlueprintResources/StandardMacros.IsValid` _actualcomponent_2
    (:`Is Valid`
      (remove `AudioComponent.OnAudioFinished` _actualcomponent_2 (`|CreateDelegate` :!event `OnHuntMusicFinished`)))
    (:`Is Not Valid`
      _))
  (`self.stopMusic`)
  (`self.HISetCombatMusic` (make `DataTableRowHandle` "/Game/Logic/DataTables/CDT_Audio.CDT_Audio" (`self.Combat Music Intro`)))
  (if (`KismetSystemLibrary.IsValid` _actualcomponent)
    (`AudioComponent.FadeOut` _actualcomponent 1.5 0.0 "Logarithmic"))
  (`self.HIPlayMusic` "CombatMusic" (`self.combatMusic`) 0.7)
  (add `AudioComponent.OnAudioFinished` (`self.actualComponent`) (`|CreateDelegate` :!event `OnCombatMusicFinished`)))

(event `OnCombatMusicFinished`
  (`self.stopMusic`)
  (`self.HISetCombatMusic` (make `DataTableRowHandle` "/Game/Logic/DataTables/CDT_Audio.CDT_Audio" (`self.Combat Music Loop`)))
  (`self.HIPlayMusic` "CombatMusic" (`self.combatMusic`))
  (remove `AudioComponent.OnAudioFinished` (`self.actualComponent`) (`|CreateDelegate` :!event `OnCombatMusicFinished`)))

(event `self.HIPlayHunt`
  (bind _actualcomponent (`self.actualComponent`))
  (bind _actualcomponent_2 (`self.actualComponent`))
  (`/Engine/EditorBlueprintResources/StandardMacros.IsValid` _actualcomponent
    (:`Is Valid`
      (remove `AudioComponent.OnAudioFinished` _actualcomponent (`|CreateDelegate` :!event `OnCombatMusicFinished`)))
    (:`Is Not Valid`
      _))
  (`self.stopMusic`)
  (`self.HISetHuntMusic` (make `DataTableRowHandle` "/Game/Logic/DataTables/CDT_Audio.CDT_Audio" (`self.Hunt Music Intro`)))
  (if (`KismetSystemLibrary.IsValid` _actualcomponent_2)
    (`AudioComponent.FadeOut` _actualcomponent_2 1.5 0.0 "Logarithmic"))
  (`self.HIPlayMusic` "HuntMusic" (`self.huntMusic`) 0.7)
  (add `AudioComponent.OnAudioFinished` (`self.actualComponent`) (`|CreateDelegate` :!event `OnHuntMusicFinished`)))

(event `stopMusic`
  (bind _actualcomponent (`self.actualComponent`))
  (if (`KismetSystemLibrary.IsValid` _actualcomponent)
    (`AudioComponent.Stop` _actualcomponent)))

(event `OnHuntMusicFinished`
  (`self.stopMusic`)
  (`self.HISetHuntMusic` (make `DataTableRowHandle` "/Game/Logic/DataTables/CDT_Audio.CDT_Audio" (`self.Hunt Music Loop`)))
  (`self.HIPlayMusic` "HuntMusic" (`self.huntMusic`))
  (remove `AudioComponent.OnAudioFinished` (`self.actualComponent`) (`|CreateDelegate` :!event `OnHuntMusicFinished`)))

(event `self.HIPlayPause`
  (`KismetSystemLibrary.PrintString` "MusicPause UwU"))

(fn `BridgeSoundtrack`
  (set `self.Hunt Music Loop` "Chase_Music_1_Loop")
  (set `self.Hunt Music Outro` "Chase_Music_1_Outro")
  (set `self.Combat Music Loop` "Combat_Music_2_Loop")
  (set `self.Combat Music Outro` "Combat_Music_2_Outro"))

(fn `ChangeCurrentSoundtrack`
  (params (`New Hunt Music` :type Name) (`New Combat Music` :type Name))
  (if (not (== `New Hunt Music` `New Combat Music`))
    (set `self.Hunt Music Intro` `New Hunt Music`)
    (bind _output_get (set `self.Combat Music Intro` `New Combat Music`))
    (if (== _output_get "Combat_Music_2_Intro")
      (`self.BridgeSoundtrack`)
      (else
        (`self.HunterSoundtrack`)))))

(fn `HunterSoundtrack`
  (set `self.Hunt Music Loop` "Hunt_Music_1_Loop")
  (set `self.Hunt Music Outro` "Hunt_Music_1_Outro")
  (set `self.Combat Music Loop` "FinalBoss_Music_Loop")
  (set `self.Combat Music Outro` "FinalBoss_Music_Outro"))

(fn `UserConstructionScript`)